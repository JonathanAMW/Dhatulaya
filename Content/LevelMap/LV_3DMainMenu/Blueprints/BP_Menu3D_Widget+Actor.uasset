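; Actor for a 3D main menu that hosts a widget and moves the player's view between linked menu actors.
; On BeginPlay it binds to the widget's transition event and disables its own collision.
; A valid menu index triggers TransitionTo, which swaps collision to the target menu and blends the view target to it with ease-in-out.
; The TransitionTo call shows no target argument, and the indexed LinkedMenus lookup is unused.
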(event `self.ReceiveBeginPlay`
  (bind _asmenu_3d_widget (cast `/Game/LevelMap/LV_3DMainMenu/Widgets/Menu3D_Widget` (`WidgetComponent.GetUserWidgetObject` (`self.Widget_0`))))
  (add `/Game/LevelMap/LV_3DMainMenu/Widgets/Menu3D_Widget.TransitionToLinkedMenu` _asmenu_3d_widget (delegate `OnTransitionBetweenMenu`))
  (`self.SetActorEnableCollision` false))

(event `OnTransitionBetweenMenu`
  (params (MenuIndex :type Integer))
  (if (`KismetArrayLibrary.Array_IsValidIndex` (`self.LinkedMenus_0`) MenuIndex)
    (`self.TransitionTo` null)))

(event `TransitionTo`
  (params (NewMenu :type "/Game/LevelMap/LV_3DMainMenu/Blueprints/BP_Menu3D_Widget+Actor Object Reference"))
  (`self.SetActorEnableCollision` false)
  (`self.SetActorEnableCollision` NewMenu true)
  (`PlayerController.SetViewTargetWithBlend` (`GameplayStatics.GetPlayerController` 0) NewMenu 2.0 "VTBlend_EaseInOut" 2.0 false))

(fn `UserConstructionScript`)
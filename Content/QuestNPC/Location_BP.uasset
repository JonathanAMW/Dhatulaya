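; Quest location trigger actor that completes a player's active quest when BP_MainChara enters its Box volume.
; On overlap it searches the player's ActiveQuests for entries whose ActorReference is this actor and calls QuestComplete on each match.
; It then scans all BP_QuestNPC actors and fires EventQuestComplete on those with the same quest name, linking them by name rather than by direct reference.
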(event `self.Box.OnComponentBeginOverlap`
  (params (OverlappedComponent :type "PrimitiveComponent Object Reference") (OtherActor :type "Actor Object Reference") (OtherComp :type "PrimitiveComponent Object Reference") (OtherBodyIndex :type Integer) (bFromSweep :type Boolean) (SweepResult :type "HitResult Structure (by ref)"))
  (bind _asbp_main_chara (cast `/Game/Characters/Player/Blueprints/BP_MainChara` OtherActor))
  (for _array_element (`/Game/Characters/Player/Blueprints/BP_MainChara.ActiveQuests` _asbp_main_chara)
    (bind (_questinfo_questname _questinfo_questdescription _questinfo_actorreference) (break `/Game/QuestNPC/QuestInfo` (`/Game/QuestNPC/BP_Quest.QuestInfo` _array_element)))
    (if (== self _questinfo_actorreference)
      (`/Game/Characters/Player/Blueprints/BP_MainChara.QuestComplete` _asbp_main_chara _array_element)
      (bind _outactors (`GameplayStatics.GetAllActorsOfClass` "/Game/QuestNPC/BP_QuestNPC.BP_QuestNPC_C"))
      (for _array_element_2 _outactors
        (bind _questref_questname (break `/Game/QuestNPC/QuestInfo` (`/Game/QuestNPC/BP_QuestNPC.QuestRef` _array_element_2)))
        (if (`KismetTextLibrary.EqualEqual_TextText` _questref_questname _questinfo_questname)
          (`/Game/QuestNPC/BP_QuestNPC.EventQuestComplete` _array_element_2))))))

(fn `UserConstructionScript`)